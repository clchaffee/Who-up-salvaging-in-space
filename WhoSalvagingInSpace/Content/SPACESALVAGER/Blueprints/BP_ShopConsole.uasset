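; BP_ShopConsole is a shop console actor that tracks when the player is within range of it.
; Its TriggerZone overlap events cast to BP_FirstPersonCharacter and set that character's IsNearShop flag on entry, clearing it on exit.
; Disconnected nodes for toggling input and opening the WPB_ShopUI widget with a mouse cursor never run, so the console itself does not open the shop.
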(event `self.TriggerZone.OnComponentBeginOverlap`
  (params (OverlappedComponent :type "PrimitiveComponent Object Reference") (OtherActor :type "Actor Object Reference") (OtherComp :type "PrimitiveComponent Object Reference") (OtherBodyIndex :type Integer) (bFromSweep :type Boolean) (SweepResult :type "HitResult Structure (by ref)"))
  (bind _asbp_first_person_character (cast `/Game/SPACESALVAGER/Blueprints/BP_FirstPersonCharacter` OtherActor))
  (set `/Game/SPACESALVAGER/Blueprints/BP_FirstPersonCharacter.IsNearShop` true _asbp_first_person_character))

(event `Key|E`
  (params (Key :type "Key Structure")))

(event `self.TriggerZone.OnComponentEndOverlap`
  (params (OverlappedComponent :type "PrimitiveComponent Object Reference") (OtherActor :type "Actor Object Reference") (OtherComp :type "PrimitiveComponent Object Reference") (OtherBodyIndex :type Integer))
  (bind _asbp_first_person_character (cast `/Game/SPACESALVAGER/Blueprints/BP_FirstPersonCharacter` OtherActor))
  (set `/Game/SPACESALVAGER/Blueprints/BP_FirstPersonCharacter.IsNearShop` false _asbp_first_person_character))

(fn `UserConstructionScript`)