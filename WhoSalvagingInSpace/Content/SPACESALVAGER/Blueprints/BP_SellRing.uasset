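; BP_SellRing is a ring that sells objects thrown through it and kills the player who passes through.
; When anything other than the player stops overlapping its cylinder, it grants the player a fixed amount of Spacebux, destroys the object and plays a sale sound.
; When the player exits the cylinder, a guarded branch plays a sound, holds the screen faded out, then reloads the space level after a short delay.
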(event `self.ReceiveBeginPlay`
  (bind _returnvalue (`GameplayStatics.GetActorOfClass` "/Game/SPACESALVAGER/Blueprints/BP_FirstPersonCharacter.BP_FirstPersonCharacter_C"))
  (set `self.PlayerRef` _returnvalue))

(event `self.Cylinder.OnComponentEndOverlap`
  (params (OverlappedComponent :type "PrimitiveComponent Object Reference") (OtherActor :type "Actor Object Reference") (OtherComp :type "PrimitiveComponent Object Reference") (OtherBodyIndex :type Integer))
  ; Destroy whatever you throw in as long as it's NOT a player
  (`KismetSystemLibrary.PrintString` "RingDetectsObj" true true (struct :`R` 0.852431 :`G` 0.532386 :`B` 0.005828 :`A` 1.0))
  (cast `/Game/SPACESALVAGER/Blueprints/BP_FirstPersonCharacter` OtherActor
    (:`then`
      (`self.ShouldStopDeathStacks`
        (:`then`)
        (:`else`
          (`GameplayStatics.PlaySound2D` "/Game/SPACESALVAGER/Audio/Sfx/FNAF.FNAF" 1.0 1.0 0.0 null null)
          (`PlayerCameraManager.StartCameraFade` :`self` (`PlayerController.PlayerCameraManager` (`GameplayStatics.GetPlayerController` 0)) :`FromAlpha` 1.0 :`ToAlpha` 1.0 :`Duration` 1.0)
          (set `self.ShouldStopDeathStacks` true)
          (`KismetSystemLibrary.Delay` 0.5)
          (`GameplayStatics.OpenLevelBySoftObjectPtr` "/Game/SPACESALVAGER/LEVELSPACE.LEVELSPACE"))))
    (:`CastFailed`
      (`/Game/SPACESALVAGER/Blueprints/BP_FirstPersonCharacter.GiveSpacebux` (`self.PlayerRef`) 5)
      (`self.K2_DestroyActor` OtherActor) ; AFTER: Call sell method
      (`GameplayStatics.SpawnSoundAtLocation` "/Game/SPACESALVAGER/Audio/Sfx/SellBuy.SellBuy" (`SceneComponent.K2_GetComponentLocation` (`self.SM_RIng`)) (struct) 1.0 1.0 0.0 null null))))

(fn `UserConstructionScript`)