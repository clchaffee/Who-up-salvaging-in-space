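; Mesh-based component for a cut point on a salvageable part, which breaks once accumulated cut progress reaches its health.
; Cut adds strength and wakes Tick, which decays progress while not being cut, drives a material heat glow and sleeps again at zero.
; On completion it stops ticking, plays break sound and effect once, and fires the CutPointDestroyed dispatcher.
; A leftover debug print runs every tick.
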(event `self.ReceiveBeginPlay`)

(event `self.ReceiveTick`
  (params (DeltaSeconds :type "Float (single-precision)"))
  (bind _returnvalue (`self.K2_GetComponentLocation`))
  ; Get Cut Progress while tick enabled
  (`KismetSystemLibrary.PrintString` "Hello")
  (if (>= (`self.CutProgress`) (`self.PartHealth`))
    ; Cut Registers as completed
    (`self.SetComponentTickEnabled` false)
    (`/Engine/EditorBlueprintResources/StandardMacros.DoOnce` false
      (:`Completed`
        (`GameplayStatics.SpawnSoundAtLocation` "/Game/SPACESALVAGER/Audio/Sfx/PartBreak.PartBreak" _returnvalue (struct) 1.0 1.0 0.0 null null)
        (`NiagaraFunctionLibrary.SpawnSystemAtLocation` "/Game/SPACESALVAGER/Niagara/Breakage.Breakage" _returnvalue)
        (`self.CutPointDestroyed` self)))
    (else
      ; Not done cutting yet, are we still being cut?
      (if (not (`self.BeingCut`))
        ; Return Cut Progress
        (set `self.CutProgress` (`KismetMathLibrary.FClamp` (- (`self.CutProgress`) 1.0) 0.0 100.0)))
      ; Heat Glow
      (`self.SetScalarParameterValueOnMaterials` "CutProgress" (/ (`self.CutProgress`) (`self.PartHealth`)))
      ; Stop Tick
      (if (<= (`self.CutProgress`) 0.0)
        (`self.SetComponentTickEnabled` false)))))

(event `Cut`
  (params (`Cutting Strength` :type "Float (double-precision)"))
  (set `self.CutProgress` (+ `Cutting Strength` (`self.CutProgress`)))
  (if (not (`self.IsComponentTickEnabled`))
    (`self.SetComponentTickEnabled` true)))