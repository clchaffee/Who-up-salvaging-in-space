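; BP_Glorp is a one-shot triggered actor that plays a Glorp sound and then moves when the first-person player enters its Box.
; Tick starts disabled; the first player overlap plays the sound, waits briefly, then enables Tick.
; Each Tick sets the root's transform to the Billboard's location plus a fixed world X offset, a frame-rate-dependent step with no stop condition.
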(event `self.ReceiveBeginPlay`
  (`self.SetActorTickEnabled` false))

(event `self.Box.OnComponentBeginOverlap`
  (params (OverlappedComponent :type "PrimitiveComponent Object Reference") (OtherActor :type "Actor Object Reference") (OtherComp :type "PrimitiveComponent Object Reference") (OtherBodyIndex :type Integer) (bFromSweep :type Boolean) (SweepResult :type "HitResult Structure (by ref)"))
  (cast `/Game/SPACESALVAGER/Blueprints/BP_FirstPersonCharacter` OtherActor)
  (`/Engine/EditorBlueprintResources/StandardMacros.DoOnce` false
    (:`Completed`
      (`GameplayStatics.PlaySoundAtLocation` "/Game/SPACESALVAGER/Audio/Sfx/Glorp.Glorp" (0.0 0.0 0.0) (struct) 0.3 1.0 0.0 null null null null)
      (`KismetSystemLibrary.Delay` 3.0)
      (`self.SetActorTickEnabled` true))))

(event `self.ReceiveTick`
  (params (DeltaSeconds :type "Float (single-precision)"))
  (bind _returnvalue_location (`KismetMathLibrary.BreakTransform` (`SceneComponent.K2_GetComponentToWorld` (`self.Billboard`))))
  (`SceneComponent.K2_SetWorldTransform` (`self.DefaultSceneRoot`) (`KismetMathLibrary.MakeTransform` (+ _returnvalue_location (30.0 0.0 0.0))) false false))

(fn `UserConstructionScript`)