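; Temporary sell ring that turns salvage leaving its cylinder trigger into Spacebux for the player.
; On end overlap it spawns a Niagara explosion, pays out the component's mass, prints its name and plays a sell sound.
; A cast chain routes removal to DestroyPart on satellite, multi-part and space ad actors, or destroys random scrap outright.
; A player passing through instead gets a death sound and blackout before LEVELSPACE opens.
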(event `self.ReceiveBeginPlay`
  (bind _returnvalue (`GameplayStatics.GetActorOfClass` "/Game/SPACESALVAGER/Blueprints/BP_FirstPersonCharacter.BP_FirstPersonCharacter_C"))
  (set `self.PlayerRef` _returnvalue))

(event `self.Cylinder.OnComponentEndOverlap`
  (params (OverlappedComponent :type "PrimitiveComponent Object Reference") (OtherActor :type "Actor Object Reference") (OtherComp :type "PrimitiveComponent Object Reference") (OtherBodyIndex :type Integer))
  ; Destroy whatever you throw in as long as it's NOT a player
  (bind _output_get (set `self.OverlapReference` OtherComp))
  (bind (_returnvalue_location _returnvalue_rotation _returnvalue_scale) (`KismetMathLibrary.BreakTransform` (`SceneComponent.K2_GetComponentToWorld` _output_get)))
  ; Does a Rocket League style goal explosion
  (`NiagaraFunctionLibrary.SpawnSystemAtLocation` "/Game/SPACESALVAGER/Niagara/NS_SellExplosion.NS_SellExplosion" _returnvalue_location (struct :`Pitch` 90.0) _returnvalue_scale)
  (cast `/Game/SPACESALVAGER/Blueprints/BP_FirstPersonCharacter` OtherActor
    (:`then`
      (`self.ShouldStopDeathStacks`
        (:`then`)
        (:`else`
          (`GameplayStatics.PlaySound2D` "/Game/SPACESALVAGER/Audio/Sfx/FNAF.FNAF" 1.0 1.0 0.0 null null)
          (`PlayerCameraManager.StartCameraFade` :`self` (`PlayerController.PlayerCameraManager` (`GameplayStatics.GetPlayerController` 0)) :`FromAlpha` 1.0 :`ToAlpha` 1.0 :`Duration` 1.0)
          (set `self.ShouldStopDeathStacks` true)
          (`KismetSystemLibrary.Delay` 0.5)
          (`GameplayStatics.OpenLevelBySoftObjectPtr` "/Game/SPACESALVAGER/LEVELSPACE.LEVELSPACE"))))
    (:`CastFailed`
      (`/Game/SPACESALVAGER/Blueprints/BP_FirstPersonCharacter.GiveSpacebux` (`self.PlayerRef`) (`KismetMathLibrary.FTrunc` (`PrimitiveComponent.GetMass` (`self.OverlapReference`))))
      (`KismetSystemLibrary.PrintString` (`KismetSystemLibrary.GetDisplayName` (`self.OverlapReference`)) true true (struct :`R` 1.0 :`B` 0.339542 :`A` 1.0))
      (`GameplayStatics.SpawnSoundAtLocation` "/Game/SPACESALVAGER/Audio/Sfx/SellBuy.SellBuy" (`SceneComponent.K2_GetComponentLocation` (`self.SM_RIng`)) (struct) 0.5 1.0 0.0 "/Game/SPACESALVAGER/Audio/DefaultSalvagedAttenuation.DefaultSalvagedAttenuation" null)
      ; Destroy any Satelite Part
      (bind _asbp_satelite (cast `/Game/SPACESALVAGER/Blueprints/BP_Satelite` OtherActor)
        (:`then`
          (`/Game/SPACESALVAGER/Blueprints/BP_Satelite.DestroyPart` _asbp_satelite (`self.OverlapReference`)))
        (:`CastFailed`
          ; Destroy Complex Satelite Part
          (bind _asbp_multiple (cast `/Game/SPACESALVAGER/Blueprints/BP_Multiple` OtherActor)
            (:`then`
              (`/Game/SPACESALVAGER/Blueprints/BP_Multiple.DestroyPart` _asbp_multiple (`self.OverlapReference`)))
            (:`CastFailed`
              (bind _asbp_space_ad (cast `/Game/SPACESALVAGER/Blueprints/BP_SpaceAd` OtherActor)
                (:`then`
                  (`/Game/SPACESALVAGER/Blueprints/BP_SpaceAd.DestroyPart` _asbp_space_ad (`self.OverlapReference`)))
                (:`CastFailed`
                  (bind _asbp_scrap_random (cast `/Game/SPACESALVAGER/Blueprints/BP_ScrapRandom` OtherActor))
                  (`self.K2_DestroyActor` _asbp_scrap_random))))))))))

(fn `UserConstructionScript`)