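; BP_SpaceAd is a salvageable space advertisement that shows a random ad and has wing parts linked to cut points.
; On BeginPlay it assigns each of three cut point components a wing, then one tick later sets the cube's material from RandomAds.
; It also prints a separately rolled ad name, which may differ from the applied one.
; A DestroyPart event destroys whichever component it receives.
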(event `self.ReceiveBeginPlay`
  (bind _outitem (`KismetArrayLibrary.Array_Random` (`self.RandomAds`)))
  (set `/Game/SPACESALVAGER/Blueprints/BP_CutPointComponent.AttachedObject` (`self.WingB`) (`self.BP_CutPointComponent1`))
  (set `/Game/SPACESALVAGER/Blueprints/BP_CutPointComponent.AttachedObject` (`self.WingA`) (`self.BP_CutPointComponent`))
  (set `/Game/SPACESALVAGER/Blueprints/BP_CutPointComponent.AttachedObject` (`self.WingA1`) (`self.BP_CutPointComponent2`))
  (`KismetSystemLibrary.DelayUntilNextTick`)
  (`PrimitiveComponent.SetMaterial` (`self.Cube`) 0 _outitem)
  (`KismetSystemLibrary.PrintString` (`KismetSystemLibrary.GetDisplayName` _outitem)))

(event `DestroyPart`
  (params (PartToDestroy :type "SceneComponent Object Reference"))
  (`ActorComponent.K2_DestroyComponent` PartToDestroy))

(fn `UserConstructionScript`)