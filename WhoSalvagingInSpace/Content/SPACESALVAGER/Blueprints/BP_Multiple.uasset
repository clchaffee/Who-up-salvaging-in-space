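; BP_Multiple is a salvageable object in Space Salvager with several detachable parts, such as wings, that can be removed at cut points.
; On BeginPlay it assigns three wing components as the attached objects of its three cut point components.
; Its DestroyPart event destroys whichever component is passed to it.
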(event `self.ReceiveBeginPlay`
  (set `/Game/SPACESALVAGER/Blueprints/BP_CutPointComponent.AttachedObject` (`self.WingB`) (`self.BP_CutPointComponent1`))
  (set `/Game/SPACESALVAGER/Blueprints/BP_CutPointComponent.AttachedObject` (`self.WingA`) (`self.BP_CutPointComponent`))
  (set `/Game/SPACESALVAGER/Blueprints/BP_CutPointComponent.AttachedObject` (`self.WingA1`) (`self.BP_CutPointComponent2`)))

(event `DestroyPart`
  (params (PartToDestroy :type "SceneComponent Object Reference"))
  (`ActorComponent.K2_DestroyComponent` PartToDestroy))

(fn `UserConstructionScript`)