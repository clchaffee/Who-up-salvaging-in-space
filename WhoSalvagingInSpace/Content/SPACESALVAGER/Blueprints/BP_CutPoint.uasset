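; Cuttable point that breaks off once accumulated cut progress reaches its part health, apparently on a salvageable satellite.
; Cut adds cutting strength to the progress, which Tick decays whenever BeingCut is false.
; Tick writes the progress ratio to a Material Parameter Collection for glow, a value shared across instances.
; On breaking, it calls CheckPoints on the first BP_SateliteMaster found, plays break sound and effects, then destroys itself.
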(event `self.ReceiveTick`
  (params (DeltaSeconds :type "Float (single-precision)"))
  (bind _returnvalue (`SceneComponent.K2_GetComponentLocation` (`self.Cube`)))
  (if (>= (`self.CutProgress`) (`self.PartHealth`))
    (bind _returnvalue_2 (`GameplayStatics.GetActorOfClass` "/Game/SPACESALVAGER/Blueprints/BP_SateliteMaster.BP_SateliteMaster_C"))
    (`/Game/SPACESALVAGER/Blueprints/BP_SateliteMaster.CheckPoints` _returnvalue_2)
    (`self.SetActorHiddenInGame` true)
    (`GameplayStatics.SpawnSoundAtLocation` "/Game/SPACESALVAGER/Audio/Sfx/PartBreak.PartBreak" _returnvalue (struct) 1.0 1.0 0.0 null null)
    (`NiagaraFunctionLibrary.SpawnSystemAtLocation` "/Game/SPACESALVAGER/Niagara/Breakage.Breakage" _returnvalue)
    (`self.K2_DestroyActor`) ; Only here for now, will require detaching parts first later
    (else
      (if (not (`self.BeingCut`))
        (set `self.CutProgress` (`KismetMathLibrary.FClamp` (- (`self.CutProgress`) 1.0) 0.0 100.0)))
      (`KismetMaterialLibrary.SetScalarParameterValue` "/Game/SPACESALVAGER/Materials/MPC_CutPointGlowStrength.MPC_CutPointGlowStrength" "CutProgress" (/ (`self.CutProgress`) (`self.PartHealth`))))))

(event `Cut`
  (params (`Cutting Strength` :type "Float (double-precision)"))
  (bind _output_get (set `self.CutProgress` (+ `Cutting Strength` (`self.CutProgress`))))
  (`KismetSystemLibrary.PrintString` (`KismetStringLibrary.Conv_DoubleToString` _output_get)))

(fn `UserConstructionScript`)