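; BP_CutPointComponent is a cut point in a salvage game that breaks an attached part free once enough cutting is applied.
; Cut adds strength to CutProgress and wakes Tick, which decays progress when not being cut, drives glow through a Material Parameter Collection and sleeps at zero.
; Reaching PartHealth plays break sound and Niagara effect, enables physics on AttachedObject, radially pushes it and the parent, then destroys the component.
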(event `self.ReceiveBeginPlay`)

(event `self.ReceiveTick`
  (params (DeltaSeconds :type "Float (single-precision)"))
  (bind _returnvalue (`self.K2_GetComponentLocation`))
  (if (>= (`self.CutProgress`) (`self.PartHealth`))
    (`self.SetComponentTickEnabled` false)
    (`/Engine/EditorBlueprintResources/StandardMacros.DoOnce` false
      (:`Completed`
        (`GameplayStatics.SpawnSoundAtLocation` "/Game/SPACESALVAGER/Audio/Sfx/PartBreak.PartBreak" _returnvalue (struct) 1.0 1.0 0.0 null null)
        (`NiagaraFunctionLibrary.SpawnSystemAtLocation` "/Game/SPACESALVAGER/Niagara/Breakage.Breakage" _returnvalue)
        (`self.SetSimulatePhysics` (`self.AttachedObject`) true)
        (`PhysicsObjectBlueprintLibrary.ApplyRadialImpulse` (`self.AttachedObject`) (`self.K2_GetComponentLocation`) 1000.0 250.0 "RIF_Constant" false 0.0 true)
        (`PhysicsObjectBlueprintLibrary.ApplyRadialImpulse` (cast `PrimitiveComponent` (`|GetArrayItem` (`self.GetParentComponents`)) :!pure true) (`self.K2_GetComponentLocation`) 1000.0 250.0 "RIF_Constant" false 0.0 true)
        (`self.K2_DestroyComponent`)))
    (else
      (if (not (`self.BeingCut`))
        ; Return Cut Progress
        (set `self.CutProgress` (`KismetMathLibrary.FClamp` (- (`self.CutProgress`) 1.0) 0.0 100.0)))
      ; Heat Glow
      (`KismetMaterialLibrary.SetScalarParameterValue` "/Game/SPACESALVAGER/Materials/MPC_CutPointGlowStrength.MPC_CutPointGlowStrength" "CutProgress" (/ (`self.CutProgress`) (`self.PartHealth`)))
      ; Stop Tick
      (if (<= (`self.CutProgress`) 0.0)
        (`self.SetComponentTickEnabled` false)))))

(event `Cut`
  (params (`Cutting Strength` :type "Float (double-precision)"))
  (bind _output_get (set `self.CutProgress` (+ `Cutting Strength` (`self.CutProgress`))))
  (`KismetSystemLibrary.PrintString` (`KismetStringLibrary.Conv_DoubleToString` _output_get) true true (struct :`R` 1.0 :`G` 0.902835 :`A` 1.0) 0.1)
  (if (not (`self.IsComponentTickEnabled`))
    (`self.SetComponentTickEnabled` true)))