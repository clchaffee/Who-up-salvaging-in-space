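; Deprecated Space Salvager Blueprint for an object with five panels, each linked to a cut point.
; On BeginPlay it assigns each of the five BPCutPointComponents its panel, A through E, as the AttachedObject.
; A DestroyPart event destroys whichever component is passed to it; nothing in this graph calls it, and the construction script is empty.
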(event `self.ReceiveBeginPlay`
  (set `/Game/SPACESALVAGER/Blueprints/Depricated/BP_CutPointComponentLessOld.AttachedObject` (`self.PANELB`) (`self.BP_CutPointComponent1`))
  (set `/Game/SPACESALVAGER/Blueprints/Depricated/BP_CutPointComponentLessOld.AttachedObject` (`self.PANELA`) (`self.BP_CutPointComponent`))
  (set `/Game/SPACESALVAGER/Blueprints/Depricated/BP_CutPointComponentLessOld.AttachedObject` (`self.PANELC`) (`self.BP_CutPointComponent2`))
  (set `/Game/SPACESALVAGER/Blueprints/Depricated/BP_CutPointComponentLessOld.AttachedObject` (`self.PANELD`) (`self.BP_CutPointComponent3`))
  (set `/Game/SPACESALVAGER/Blueprints/Depricated/BP_CutPointComponentLessOld.AttachedObject` (`self.PANELE`) (`self.BP_CutPointComponent4`)))

(event `DestroyPart`
  (params (PartToDestroy :type "SceneComponent Object Reference"))
  (`ActorComponent.K2_DestroyComponent` PartToDestroy))

(fn `UserConstructionScript`)