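; BP_GravityZone is a box volume that switches the first-person player between gravity and zero-gravity movement.
; On BeginPlay it caches the BP_FirstPersonCharacter, and its overlap events respond only to that actor.
; Entering calls SetMovementMode(false) and reorients the player for gravity, while leaving calls SetMovementMode(true).
; Both crossings play a random zero-gravity barrier sound at the player's mesh.
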(event `self.ReceiveBeginPlay`
  (bind _returnvalue (`GameplayStatics.GetActorOfClass` "/Game/SPACESALVAGER/Blueprints/BP_FirstPersonCharacter.BP_FirstPersonCharacter_C"))
  (set `self.PlayerRef` _returnvalue))

(event `self.Box.OnComponentBeginOverlap`
  (params (OverlappedComponent :type "PrimitiveComponent Object Reference") (OtherActor :type "Actor Object Reference") (OtherComp :type "PrimitiveComponent Object Reference") (OtherBodyIndex :type Integer) (bFromSweep :type Boolean) (SweepResult :type "HitResult Structure (by ref)"))
  (bind _playerref (`self.PlayerRef`))
  (if (== OtherActor (`self.PlayerRef`))
    (`GameplayStatics.SpawnSoundAtLocation` (`KismetArrayLibrary.Array_Random` (`self.ZeroGravityBarrierSounds`)) (`SceneComponent.K2_GetComponentLocation` (`Character.Mesh` _playerref)) (struct) 1.0 1.0 0.0 null null)
    (`/Game/SPACESALVAGER/Blueprints/BP_FirstPersonCharacter.SetMovementMode` _playerref false)
    (`/Game/SPACESALVAGER/Blueprints/BP_FirstPersonCharacter.ReorientInGavity` (`self.PlayerRef`))))

(event `self.Box.OnComponentEndOverlap`
  (params (OverlappedComponent :type "PrimitiveComponent Object Reference") (OtherActor :type "Actor Object Reference") (OtherComp :type "PrimitiveComponent Object Reference") (OtherBodyIndex :type Integer))
  (bind _playerref (`self.PlayerRef`))
  (if (== OtherActor (`self.PlayerRef`))
    (`GameplayStatics.SpawnSoundAtLocation` (`KismetArrayLibrary.Array_Random` (`self.ZeroGravityBarrierSounds`)) (`SceneComponent.K2_GetComponentLocation` (`Character.Mesh` _playerref)) (struct) 1.0 1.0 0.0 null null)
    (`/Game/SPACESALVAGER/Blueprints/BP_FirstPersonCharacter.SetMovementMode` _playerref true)))

(fn `UserConstructionScript`)