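; BP_Ads is a salvageable ad billboard built on a parent salvage Blueprint, apparently meant as a duplicable example.
; On BeginPlay it fills three cut points' attached-object arrays, linking two thrusters and an antenna to the board.
; It then applies a random material from RandomAds to the image.
; The debug print makes a separate random pick, so its name may differ from the displayed ad.
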(event `self.ReceiveBeginPlay`
  (bind _outitem (`KismetArrayLibrary.Array_Random` (`self.RandomAds`)))
  ;[0.15 0 0.009531 0.5] DUPLICATE THIS BP. IT MUST Maintain its Parent.
  (`parent.ReceiveBeginPlay`)
  ; Example Setup Explanation
  (set `/Game/SPACESALVAGER/Blueprints/BP_CutPointComponentNewSystem.AttachedObject` (`|MakeArray` (`self.ThrustB`) (`self.Board`)) (`self.CP-B`)) ; This is the array of attached objects\n<--- Read this
  ; Attach Wing A to Core
  (set `/Game/SPACESALVAGER/Blueprints/BP_CutPointComponentNewSystem.AttachedObject` (`|MakeArray` (`self.ThrustA`) (`self.Board`)) (`self.CP-A`)) ; Repeat this process for EVERY connect object\nusing this format
  (set `/Game/SPACESALVAGER/Blueprints/BP_CutPointComponentNewSystem.AttachedObject` (`|MakeArray` (`self.Board`) (`self.AntennaC`)) (`self.CP-C`)) ; Repeat this process for EVERY connect object\nusing this format
  (`PrimitiveComponent.SetMaterial` (`self.Image`) 0 _outitem)
  (`KismetSystemLibrary.PrintString` (`KismetSystemLibrary.GetDisplayName` _outitem)))

(fn `UserConstructionScript`)