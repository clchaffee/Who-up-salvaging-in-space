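; BP_Rover is a salvageable rover that also serves as a template to duplicate for other salvage objects, keeping the same parent.
; BeginPlay runs the parent logic, then fills each cut point's AttachedObject array with the two parts it connects.
; Two cut points join the body halves, while others link the solar panel, dish arm and four wheels to their body half.
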(event `self.ReceiveBeginPlay`
  ;[0.15 0 0.009531 0.5] DUPLICATE THIS BP. IT MUST Maintain its Parent.
  (`parent.ReceiveBeginPlay`)
  ; Example Setup Explanation
  (set `/Game/SPACESALVAGER/Blueprints/BP_CutPointComponentNewSystem.AttachedObject` (`|MakeArray` (`self.BodyLeft`) (`self.BodyRight`)) (`self.CPBody2`)) ; This is the array of attached objects\n<--- Read this
  ; Attach Body Bits, Again
  (set `/Game/SPACESALVAGER/Blueprints/BP_CutPointComponentNewSystem.AttachedObject` (`|MakeArray` (`self.BodyLeft`) (`self.BodyRight`)) (`self.CPBody1`)) ; Repeat this process for EVERY connect object\nusing this format
  (set `/Game/SPACESALVAGER/Blueprints/BP_CutPointComponentNewSystem.AttachedObject` (`|MakeArray` (`self.SolarPanel`) (`self.BodyRight`)) (`self.CPSolarPanel`)) ; Repeat this process for EVERY connect object\nusing this format
  (set `/Game/SPACESALVAGER/Blueprints/BP_CutPointComponentNewSystem.AttachedObject` (`|MakeArray` (`self.BodyLeft`) (`self.DishArm`)) (`self.CPDIshArm`))
  (set `/Game/SPACESALVAGER/Blueprints/BP_CutPointComponentNewSystem.AttachedObject` (`|MakeArray` (`self.Wheel1`) (`self.BodyLeft`)) (`self.CPWheel1`))
  (set `/Game/SPACESALVAGER/Blueprints/BP_CutPointComponentNewSystem.AttachedObject` (`|MakeArray` (`self.Wheel3`) (`self.BodyLeft`)) (`self.CPWheel3`))
  (set `/Game/SPACESALVAGER/Blueprints/BP_CutPointComponentNewSystem.AttachedObject` (`|MakeArray` (`self.Wheel2`) (`self.BodyRight`)) (`self.CPWheel2`))
  (set `/Game/SPACESALVAGER/Blueprints/BP_CutPointComponentNewSystem.AttachedObject` (`|MakeArray` (`self.Wheel4`) (`self.BodyRight`)) (`self.CPWheel4`)))

(fn `UserConstructionScript`)