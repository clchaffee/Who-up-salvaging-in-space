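; BP_SateliteNewSystem is a satellite Blueprint that doubles as a template to duplicate for new objects, keeping the same parent class.
; On BeginPlay it runs the parent logic, then fills each cut point's AttachedObjects array with the two pieces it connects.
; CPWingA and CPWingB link WingA and WingB to the shared Core, an example of the setup repeated for every connection.
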(event `self.ReceiveBeginPlay`
  ;[0.15 0 0.009531 0.5] DUPLICATE THIS BP. IT MUST Maintain its Parent.
  (`parent.ReceiveBeginPlay`)
  ; Example Setup Explanation
  (set `/Game/SPACESALVAGER/Blueprints/BP_CutPointComponentNewSystem.AttachedObjects` (`|MakeArray` (`self.WingB`) (`self.Core`)) (`self.CPWingB`)) ; This is the array of attached objects\n<--- Read this
  ; Attach Wing A to Core
  (set `/Game/SPACESALVAGER/Blueprints/BP_CutPointComponentNewSystem.AttachedObjects` (`|MakeArray` (`self.WingA`) (`self.Core`)) (`self.CPWingA`)) ; Repeat this process for EVERY connect object\nusing this format
)

(fn `UserConstructionScript`)