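; BP_SolarArray is a salvageable solar array made of solar pieces, a dish arm and a control panel around a central core.
; On BeginPlay it calls its parent, then gives each cut point the pair of objects it connects: one outer part and the core.
; It serves as a duplication template whose comments explain this pairing format, and copies must keep the same parent class.
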(event `self.ReceiveBeginPlay`
  ;[0.15 0 0.009531 0.5] DUPLICATE THIS BP. IT MUST Maintain its Parent.
  (`parent.ReceiveBeginPlay`)
  ; Example Setup Explanation
  (set `/Game/SPACESALVAGER/Blueprints/BP_CutPointComponentNewSystem.AttachedObject` (`|MakeArray` (`self.Solar1`) (`self.Core`)) (`self.CP1`)) ; This is the array of attached objects\n<--- Read this
  ; Attach Wing A to Core
  (set `/Game/SPACESALVAGER/Blueprints/BP_CutPointComponentNewSystem.AttachedObject` (`|MakeArray` (`self.Solar2`) (`self.Core`)) (`self.CP2`)) ; Repeat this process for EVERY connect object\nusing this format
  (set `/Game/SPACESALVAGER/Blueprints/BP_CutPointComponentNewSystem.AttachedObject` (`|MakeArray` (`self.Solar3`) (`self.Core`)) (`self.CP3`))
  (set `/Game/SPACESALVAGER/Blueprints/BP_CutPointComponentNewSystem.AttachedObject` (`|MakeArray` (`self.Solar4`) (`self.Core`)) (`self.CP4`))
  (set `/Game/SPACESALVAGER/Blueprints/BP_CutPointComponentNewSystem.AttachedObject` (`|MakeArray` (`self.Solar5`) (`self.Core`)) (`self.CP5`))
  (set `/Game/SPACESALVAGER/Blueprints/BP_CutPointComponentNewSystem.AttachedObject` (`|MakeArray` (`self.Solar6`) (`self.Core`)) (`self.CP6`))
  (set `/Game/SPACESALVAGER/Blueprints/BP_CutPointComponentNewSystem.AttachedObject` (`|MakeArray` (`self.DishArm`) (`self.Core`)) (`self.CPDish`))
  (set `/Game/SPACESALVAGER/Blueprints/BP_CutPointComponentNewSystem.AttachedObject` (`|MakeArray` (`self.ControlPanel`) (`self.Core`)) (`self.CPControl`)))

(fn `UserConstructionScript`)