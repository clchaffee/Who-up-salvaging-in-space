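; BP_FloatingBeacon is a salvageable floating beacon Blueprint, built as a child of a parent salvage class and meant to be duplicated as a template.
; On BeginPlay it runs the parent logic, then fills each connection point's AttachedObject array.
; Each connection point pairs one part, three panels and an antenna, with the central Core.
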(event `self.ReceiveBeginPlay`
  ;[0.15 0 0.009531 0.5] DUPLICATE THIS BP. IT MUST Maintain its Parent.
  (`parent.ReceiveBeginPlay`)
  ; Example Setup Explanation
  (set `/Game/SPACESALVAGER/Blueprints/BP_CutPointComponentNewSystem.AttachedObject` (`|MakeArray` (`self.Panel1`) (`self.Core`)) (`self.CPPanel1`)) ; This is the array of attached objects\n<--- Read this
  ; Attach Wing A to Core
  (set `/Game/SPACESALVAGER/Blueprints/BP_CutPointComponentNewSystem.AttachedObject` (`|MakeArray` (`self.Panel2`) (`self.Core`)) (`self.CPPanel2`)) ; Repeat this process for EVERY connect object\nusing this format
  (set `/Game/SPACESALVAGER/Blueprints/BP_CutPointComponentNewSystem.AttachedObject` (`|MakeArray` (`self.Panel3`) (`self.Core`)) (`self.CPPanel3`))
  (set `/Game/SPACESALVAGER/Blueprints/BP_CutPointComponentNewSystem.AttachedObject` (`|MakeArray` (`self.Antenna`) (`self.Core`)) (`self.CPAntenna`)))

(fn `UserConstructionScript`)