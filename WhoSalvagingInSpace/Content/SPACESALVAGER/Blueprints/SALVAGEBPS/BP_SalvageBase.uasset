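; BP_SalvageBase is a salvage object whose parts break loose when its cut points are destroyed.
; On BeginPlay it gathers its cut point components and binds their destroyed event.
; That event compares the broken point's attached objects with the other points' to build an eject list, then enables physics, applies a radial impulse and destroys the cut point.
; RemovePart destroys a given component.
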(event `self.ReceiveBeginPlay`
  (bind _output_get (set `self.CutPointList` (`self.K2_GetComponentsByClass` "/Game/SPACESALVAGER/Blueprints/BP_CutPointComponentNewSystem.BP_CutPointComponentNewSystem_C")))
  (add `/Game/SPACESALVAGER/Blueprints/BP_CutPointComponentNewSystem.CutPointDestroyed` _output_get (delegate `CutPointDestroyed_Event`)))

(event `CutPointDestroyed_Event`
  (params (CutPoint :type "/Game/SPACESALVAGER/Blueprints/BP_CutPointComponentNewSystem Object Reference"))
  (bind _ejectlist (`self.EjectList`))
  (bind _ejectlist_2 (`self.EjectList`))
  (for _array_element (`self.CutPointList`)
    (if (!= _array_element CutPoint)
      (for _array_element_2 (`/Game/SPACESALVAGER/Blueprints/BP_CutPointComponentNewSystem.AttachedObject` CutPoint)
        (`/Engine/EditorBlueprintResources/StandardMacros.IsValid` _array_element_2
          (:`Is Valid`
            (if (`KismetArrayLibrary.Array_Contains` (`/Game/SPACESALVAGER/Blueprints/BP_CutPointComponentNewSystem.AttachedObject` _array_element) _array_element_2)
              (if (`KismetArrayLibrary.Array_Contains` _ejectlist _array_element_2)
                (`KismetArrayLibrary.Array_RemoveItem` _ejectlist _array_element_2) ; Removes
              )
              (else
                (`KismetArrayLibrary.Array_Add` _ejectlist _array_element_2) ; From the list, these are\nwhat we wish to disconnect
              )))
          (:`Is Not Valid`
            (`KismetSystemLibrary.PrintString` "INVALID" true true (struct :`R` 1.0 :`B` 0.002858 :`A` 1.0)))))))
  (`PrimitiveComponent.SetSimulatePhysics` _ejectlist_2 true) ; When Completed - Parts to eject\nEnable phyics, apply force, etc
  (for _array_element_3 _ejectlist_2
    (`PhysicsObjectBlueprintLibrary.ApplyRadialImpulse` _array_element_3 (`SceneComponent.K2_GetComponentLocation` CutPoint) 1000.0 250.0 "RIF_Constant" false 0.0 true))
  (`ActorComponent.K2_DestroyComponent` CutPoint))

(event `self.RemovePart`
  (params (ComponentToRemove :type "SceneComponent Object Reference"))
  (`ActorComponent.K2_DestroyComponent` ComponentToRemove))

(fn `UserConstructionScript`)